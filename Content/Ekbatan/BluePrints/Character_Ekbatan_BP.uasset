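; Player character for the Ekbatan area that restores its placement from the game instance and handles movement and turning input.
; On BeginPlay it casts to MyGameInstance and moves itself to the stored MyTransform.
; Forward input follows control yaw, sideways input uses a fixed world Y axis rather than the facing direction, and mouse input drives controller yaw.
; Two disconnected SetActorLocationAndRotation chains never run.
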(event EventBeginPlay
  (bind _asmy_game_instance (Utilities|Casting|CastToMyGameInstance (Game|GetGameInstance)))
  (Transformation|SetActorTransform (Variables|/Game/Ekbatan/BluePrints/MyGameInstance.MyGameInstance_C|GetMyTransform _asmy_game_instance)))

(event Input|AxisEvents|InputAxisMoveForward
  (params (AxisValue :type Float%20%28single-precision%29))
  ;[0.9443 0.3838 1 1 37] Movement
  (Pawn|Input|AddMovementInput (Math|Vector|Normalize (Math|Vector|GetForwardVector (Math|Rotator|MakeRotator 0.0 0.0 (.yaw (Pawn|GetControlRotation :!class /Script/Engine.Pawn))))) AxisValue false))

(event Input|AxisEvents|InputAxisMoveRightleft
  (params (AxisValue :type Float%20%28single-precision%29))
  ;[0.9443 0.3838 1 1 37] Movement
  (Pawn|Input|AddMovementInput "0.000000,50.000000,0.000000" AxisValue false))

(event Input|AxisEvents|InputAxisMouseMove
  (params (AxisValue :type Float%20%28single-precision%29))
  (Pawn|Input|AddControllerYawInput AxisValue))

(fn ConstructionScript)